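; Bouncing projectile that damages pawns, leaves impact decals and can optionally explode.
; On each bounce the authority fires an impulse and sphere-overlaps pawns, applying damage scaled by player 0's character stats.
; Randomly rolled decals are stored in that character's DecalArray so they persist.
; When the bounce counter runs out, it optionally triggers Explode for radial force and particles, then is destroyed through MyCharacter's DestroyActorGlobal.
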(event OnProjectileBounce(ProjectileMovement)
  (params (ImpactResult :type Hit%20Result%20Structure%20%28by%20ref%29) (ImpactVelocity :type Vector%20%28by%20ref%29 :default "0, 0, 0"))
  (bind (_bblockinghit _time _location _normal _impactpoint _impactnormal) (Collision|BreakHitResult ImpactResult))
  (Networking|SwitchHasAuthority
    (:Authority
      (Class|RadialForceComponent|FireImpulse)
      (Development|PrintString "impulse")
      ;[1 1 1] limits how many decals per bullet
      (if (> (Variables|Default|Getbounce) 0)
        (Variables|Default|Setbounce (- (Variables|Default|Getbounce) 1))
        (CallFunction|SpawnDecalNetworked _impactpoint _impactnormal)
        (CallFunction|OnObstacleHit _impactpoint _impactnormal)
        (CallFunction|ApplyBulletDamage _impactpoint _impactnormal)
        (else
          (CallFunction|ApplyBulletDamage _impactpoint _impactnormal)
          (if (Variables|Default|Getexplodes)
            (CallFunction|Explode))
          (Default|DestroyActorGlobal (stale Custom|Spawn%20Decal%20Networked _asmy_character) self))))))

(event Custom|Spawn%20Decal%20Networked
  (params (Impact%20Point :type Vector :default "0, 0, 0") (Impact%20Normal :type Vector :default "0, 0, 0"))
  ;[1 1 1] Spawn Decals
  (bind _returnvalue (Rendering|Decal|SpawnDecalatLocation 0 (Variables|/Script/Engine.DecalComponent|GetDecalMaterial (Variables|Default|GetDecal1)) "100.000000,100.000000,1.000000" (Math|Transform|TransformLocation (Math|Conversions|ToTransform(Vector) (Class|KismetMathLibrary|GetDirectionVector "-200.000000,-200.000000,-200.000000" "200.000000,200.000000,200.000000")) Impact%20Point) (Math|Conversions|RotationFromXVector Impact%20Normal) 0.0))
  ;;[1 1 1] Puts in array so they dont disappear
  (bind _asmy_character (Utilities|Casting|CastToMyCharacter (Game|GetPlayerCharacter 0)))
  (Utilities|Array|Add (Variables|/Game/Blueprints/MyCharacter.MyCharacter_C|Getdecal_array _asmy_character) _returnvalue)
  (Transformation|AddLocalRotation _returnvalue (Class|KismetMathLibrary|MakeRot 0.0 0.0 (* (Math|Random|RandomFloat) 3.6e+02)) false))

(event EventOnObstacleHit
  (params (ImpactPoint :type Vector :default "0, 0, 0") (ImpactNormal :type Vector :default "0, 0, 0")))

(fn ConstructionScript
  (Rendering|Material|CreateDynamicMaterialInstance 0 0 :!class /Script/Engine.PrimitiveComponent)
  (Audio|Components|Audio|Play 0.0))

(fn ApplyBulletDamage
  (params (ImpactPoint :type Vector :default "0, 0, 0") (ImpactNormal :type Vector :default "0, 0, 0"))
  (bind _outactors (Class|KismetSystemLibrary|SphereOverlapActorsNEW 0 (Transformation|GetActorLocation) (Variables|Default|Getbullet%20radius) (Utilities|Array|MakeArray "ObjectTypeQuery3")))
  (for _array_element _outactors
    (bind _asmy_character (Utilities|Casting|CastToMyCharacter (Game|GetPlayerCharacter 0)))
    (Game|Damage|ApplyDamage _array_element (* (Variables|/Game/Blueprints/MyCharacter.MyCharacter_C|GetdamageMult _asmy_character) (Variables|/Game/Blueprints/MyCharacter.MyCharacter_C|GetDamage _asmy_character)) (Game|GetInstigatorController) self))
  (CallFunction|SpawnDecalNetworked ImpactPoint ImpactNormal)
  (CallFunction|OnObstacleHit ImpactPoint ImpactNormal))

(fn SpawnDecal
  (params (impact%20point :type Vector :default "0, 0, 0") (impact%20normal :type Vector :default "0, 0, 0"))
  ;[1 1 1] Spawn Decals
  (bind _returnvalue (Rendering|Decal|SpawnDecalatLocation 0 "/Game/BattleChairAssets/Materials/eagleDecal.eagleDecal" "100.000000,100.000000,1.000000" (Math|Transform|TransformLocation (Math|Conversions|ToTransform(Vector) (Class|KismetMathLibrary|GetDirectionVector "-200.000000,-200.000000,-200.000000" "200.000000,200.000000,200.000000")) impact%20point) (Math|Conversions|RotationFromXVector impact%20normal) 0.0))
  ;;[1 1 1] Puts in array so they dont disappear
  (bind _asmy_character (Utilities|Casting|CastToMyCharacter (Game|GetPlayerCharacter 0)))
  (Utilities|Array|Add (Variables|/Game/Blueprints/MyCharacter.MyCharacter_C|Getdecal_array _asmy_character) _returnvalue)
  (Transformation|AddLocalRotation _returnvalue (Class|KismetMathLibrary|MakeRot 0.0 0.0 (* (Math|Random|RandomFloat) 3.6e+02)) false))

(fn Explode
  ;[1 1 1] Makes the projectile explode and emit an explosion/sound and then damage
  (Components|DestroyComponent)
  (Components|DestroyComponent) ; Do we want this?
  (Utilities|FlowControl|DoOnce false
    (:Completed
      (Class|RadialForceComponent|FireImpulse (Variables|Default|GetRadialForce))
      (Effects|SpawnEmitteratLocation 0 (Variables|/Script/Engine.ParticleSystemComponent|GetTemplate (Variables|Default|GetParticleSystem)) (Transformation|GetActorLocation))
      (Audio|Components|Audio|Play 0.0))))