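; Burrito2 is a burrito projectile actor that tumbles until it hits an obstacle.
; The construction script picks a random spin step for each rotation axis, which Tick applies as a local rotation every frame, without delta-time scaling.
; OnObstacleHit sets a hit flag that stops the spin and sets the projectile movement's gravity scale to a small value.
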(event EventTick
  (params (DeltaSeconds :type Float%20%28single-precision%29))
  (if (not (Variables|Default|Getburritohit))
    (Transformation|AddLocalRotation (Class|KismetMathLibrary|MakeRot (Variables|Default|Getburritopitch) (Variables|Default|Getburritoyaw) (Variables|Default|Getburritoroll)) false)))

(event EventOnObstacleHit
  (params (ImpactPoint :type Vector :default "0, 0, 0") (ImpactNormal :type Vector :default "0, 0, 0"))
  (Variables|/Script/Engine.ProjectileMovementComponent|SetProjectileGravityScale (Variables|Default|GetProjectileMovement) 0.05)
  (Variables|Default|Setburritohit true))

(fn ConstructionScript
  (Variables|Default|Setburritopitch (* (Math|Random|RandomFloat) 2e+01))
  (Variables|Default|Setburritoyaw (* (Math|Random|RandomFloat) 2e+01))
  (Variables|Default|Setburritoroll (* (Math|Random|RandomFloat) 2e+01)))