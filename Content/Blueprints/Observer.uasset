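; Observer is a free-flying pawn that hides the mouse cursor and adds an ObserverHud widget on BeginPlay.
; Input events set key flags that Tick turns into movement input: WASD relative to actor facing, Space and Left Shift along world Z.
; Holding right mouse rotates the actor by the cursor's per-frame position change.
; Tick also damps velocity by a fixed divisor each frame, independent of delta time.
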(event EventBeginPlay
  (Variables|/Script/Engine.PlayerController|SetbShowMouseCursor (Game|GetPlayerController 0) false)
  (bind _returnvalue (UserInterface|CreateWidget "/Game/BattleChairAssets/HUD/ObserverHud.ObserverHud_C"))
  (UserInterface|Viewport|AddtoViewport _returnvalue 0))

(event EventActorBeginOverlap
  (params (OtherActor :type Actor%20Object%20Reference)))

(event EventTick
  (params (DeltaSeconds :type Float%20%28single-precision%29))
  (bind _returnvalue (Game|GetPlayerController 0))
  (bind _movementspeed (Variables|Default|GetmovementSpeed))
  (bind (_locationx _locationy) (Game|Player|GetMousePosition _returnvalue))
  (Variables|/Script/Engine.MovementComponent|SetVelocity (Pawn|GetMovementComponent) (/ (Transformation|GetVelocity) 1.05))
  (if (Variables|Default|Getw)
    (Pawn|Input|AddMovementInput (Math|Vector|RotateVector (Math|Vector|MakeVector 1.0 0.0 0.0) (Math|Conversions|RotationFromXVector (Transformation|GetActorForwardVector))) _movementspeed false))
  (if (Variables|Default|Geta)
    (Pawn|Input|AddMovementInput (Math|Vector|RotateVector (Math|Vector|MakeVector 0.0 -1.0 0.0) (Math|Conversions|RotationFromXVector (Transformation|GetActorForwardVector))) _movementspeed false))
  (if (Variables|Default|Gets)
    (Pawn|Input|AddMovementInput (Math|Vector|RotateVector (Math|Vector|MakeVector -1.0 0.0 0.0) (Math|Conversions|RotationFromXVector (Transformation|GetActorForwardVector))) _movementspeed false))
  (if (Variables|Default|Getd)
    (Pawn|Input|AddMovementInput (Math|Vector|RotateVector (Math|Vector|MakeVector 0.0 1.0 0.0) (Math|Conversions|RotationFromXVector (Transformation|GetActorForwardVector))) _movementspeed false))
  (Variables|Default|SetMouseX _locationx)
  (Variables|Default|SetMouseY _locationy)
  (if (Variables|Default|GetrightMouseDown)
    (Transformation|SetActorRotation (Math|Rotator|Delta(Rotator) (Transformation|GetActorRotation) (Class|KismetMathLibrary|MakeRot (- (Variables|Default|GetMouseY) (Variables|Default|GetOldMouseY)) (- (Variables|Default|GetoldMouseX) (Variables|Default|GetMouseX)) 0.0)))
    (Variables|Default|SetoldMouseX (Variables|Default|GetMouseX))
    (Variables|Default|SetOldMouseY (Variables|Default|GetMouseY)))
  (if (Variables|Default|Getl_shift)
    (Pawn|Input|AddMovementInput (Math|Vector|MakeVector 0.0 0.0 -1.0) (Variables|Default|GetmovementSpeed) false))
  (if (Variables|Default|Getspace)
    (Pawn|Input|AddMovementInput (Math|Vector|MakeVector 0.0 0.0 1.0) (Variables|Default|GetmovementSpeed) false)))

(event Input|ActionEvents|InputActionl_shift
  (:Pressed
    (Variables|Default|Setl_shift true))
  (:Released
    (Variables|Default|Setl_shift false)))

(event Input|ActionEvents|InputActionspace
  (:Pressed
    (Variables|Default|Setspace true))
  (:Released
    (Variables|Default|Setspace false)))

(event Input|ActionEvents|InputActionw
  (:Pressed
    (Variables|Default|Setw true))
  (:Released
    (Variables|Default|Setw false)))

(event Input|ActionEvents|InputActiona
  (:Pressed
    (Variables|Default|Seta true))
  (:Released
    (Variables|Default|Seta false)))

(event Input|ActionEvents|InputActiond
  (:Pressed
    (Variables|Default|Setd true))
  (:Released
    (Variables|Default|Setd false)))

(event Input|ActionEvents|InputActions
  (:Pressed
    (Variables|Default|Sets true))
  (:Released
    (Variables|Default|Sets false)))

(event Input|MouseEvents|RightMouseButton
  (:Pressed
    (Variables|Default|SetrightMouseDown true)
    (Variables|Default|SetoldMouseX (Variables|Default|GetMouseX))
    (Variables|Default|SetOldMouseY (Variables|Default|GetMouseY)))
  (:Released
    (Variables|Default|SetrightMouseDown false)))

(fn ConstructionScript)