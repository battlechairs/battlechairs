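; Credits sign actor that changes its displayed text based on the player character's CounterC value.
; Every Tick it casts the player pawn to MyCharacter, showing "Credits" at a count of zero and "Keep Looking!!" at two.
; Other counts leave the text unchanged, and a disconnected chain of numeric text updates, resembling a countdown, never runs.
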(event EventBeginPlay)

(event EventActorBeginOverlap
  (params (OtherActor :type Actor%20Object%20Reference)))

(event EventTick
  (params (DeltaSeconds :type Float%20%28single-precision%29))
  (bind _asmy_character (Utilities|Casting|CastToMyCharacter (Game|GetPlayerCharacter 0)))
  (if (== 0 (Variables|/Game/Blueprints/MyCharacter.MyCharacter_C|GetcounterC _asmy_character))
    (Rendering|Components|TextRender|SetText "Credits")
    (elif (== 2 (Variables|/Game/Blueprints/MyCharacter.MyCharacter_C|GetcounterC _asmy_character))
      (Rendering|Components|TextRender|SetText "Keep Looking!!"))))

(fn ConstructionScript)