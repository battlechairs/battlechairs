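; WarningSign is a short-lived actor, apparently a warning marker, that hovers in front of the character that instigated it.
; Every tick it casts its Instigator to MyCharacter and moves itself to a fixed forward offset, rotated by that character's rotation, without sweeping.
; It only updates location, not its own rotation, and destroys itself three seconds after BeginPlay.
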(event EventBeginPlay
  (Utilities|FlowControl|Delay 3.0)
  (Actor|DestroyActor))

(event EventActorBeginOverlap
  (params (OtherActor :type Actor%20Object%20Reference)))

(event EventTick
  (params (DeltaSeconds :type Float%20%28single-precision%29))
  (bind _asmy_character (Utilities|Casting|CastToMyCharacter (Variables|Actor|GetInstigator)))
  (Transformation|SetActorLocation (+ (Transformation|GetActorLocation _asmy_character) (Math|Vector|RotateVector (Math|Vector|MakeVector 1.2e+02 0.0 0.0) (Transformation|GetActorRotation _asmy_character))) false))

(fn ConstructionScript)