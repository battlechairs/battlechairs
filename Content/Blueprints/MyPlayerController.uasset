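; Player controller that lets a client request a respawn from the game mode.
; The Respawn action or R key, handled only without authority, calls RequestGMRespawn when no pawn is controlled, otherwise prints a debug message.
; That event acts only with authority, casting the game mode to MyGameMode and calling its Respawn with a player controller reference.
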(event Custom|requestGMRespawn
  (bind _returnvalue (Game|GetGameMode))
  ;[1 1 1] respawn character
  (Networking|SwitchHasAuthority
    (:Authority
      (Utilities|IsValid _returnvalue
        (:Is%20Valid
          (bind _asmy_game_mode (Utilities|Casting|CastToMyGameMode _returnvalue))
          (Utilities|IsValid _asmy_game_mode
            (:Is%20Valid
              (bind _returnvalue_2 (Utilities|Casting|CastToPlayerController self))
              (Default|Respawn _asmy_game_mode _returnvalue_2))))))))

(event Input|ActionEvents|InputActionRespawn
  ;[1 1 1] get keypress
  (:Pressed
    (Networking|SwitchHasAuthority
      (:Remote
        (Utilities|IsValid (Pawn|GetControlledPawn self)
          (:Is%20Valid
            (Development|PrintString "client still has pawn controlled"))
          (:Is%20Not%20Valid
            (CallFunction|RequestGMRespawn)))))))

(event Input|KeyboardEvents|R
  ;[1 1 1] get keypress
  (:Pressed
    (Networking|SwitchHasAuthority
      (:Remote
        (Utilities|IsValid (Pawn|GetControlledPawn self)
          (:Is%20Valid
            (Development|PrintString "client still has pawn controlled"))
          (:Is%20Not%20Valid
            (CallFunction|RequestGMRespawn)))))))

(fn ConstructionScript)