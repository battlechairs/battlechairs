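; Grenade launcher projectile that explodes on its first bounce, with radial force and area damage.
; The bounce runs only on authority, destroying components and using a DoOnce to fire the impulse, explosion emitter and sound.
; ApplyBulletDamage sphere-overlaps Pawns within BulletRadius, damages each, and repeats the component destruction and once-gated impulse inside that loop.
; Construction creates a dynamic material, calls Play and sets the initial speed.
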(event OnProjectileBounce(ProjectileMovement)
  (params (ImpactResult :type Hit%20Result%20Structure%20%28by%20ref%29) (ImpactVelocity :type Vector%20%28by%20ref%29 :default "0, 0, 0"))
  (Networking|SwitchHasAuthority
    (:Authority
      ;[1 1 1] Makes the projectile explode and emit an explosion/sound and then damage
      (Components|DestroyComponent)
      (Components|DestroyComponent)
      (Utilities|FlowControl|DoOnce false
        (:Completed
          (Class|RadialForceComponent|FireImpulse (Variables|Default|GetRadialForce))
          (Effects|SpawnEmitteratLocation "/Game/StarterContent/Particles/P_Explosion.P_Explosion" (Transformation|GetActorLocation))
          (Class|GameplayStatics|PlaySoundAttached "/Game/StarterContent/Audio/Explosion01.Explosion01")
          (CallFunction|ApplyBulletDamage))))))

(fn ConstructionScript
  (Rendering|Material|CreateDynamicMaterialInstance 0 0 :!class /Script/Engine.PrimitiveComponent)
  (Audio|Components|Audio|Play 0.0)
  (Variables|/Script/Engine.ProjectileMovementComponent|SetInitialSpeed (Variables|Default|GetProjectileMovement) 1e+03))

(fn ApplyBulletDamage
  (bind _outactors (Class|KismetSystemLibrary|SphereOverlapActorsNEW (Transformation|GetActorLocation) (Variables|Default|Getbullet%20radius) (Utilities|Array|MakeArray "ObjectTypeQuery3")))
  (for _array_element _outactors
    (Game|Damage|ApplyDamage _array_element (Variables|Default|GetBulletDamage) (Game|GetInstigatorController) self)
    (Components|DestroyComponent)
    (Utilities|FlowControl|DoOnce false
      (:Completed
        (Class|RadialForceComponent|FireImpulse (Variables|Default|GetRadialForce))))))