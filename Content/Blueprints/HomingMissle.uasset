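; Homing missile projectile that locks onto a character in front of player 0 and explodes on obstacle hit.
; On BeginPlay, a sphere overlap and dot-product cone test around that player's facing pick the homing target's mesh, with the last match winning.
; The construction script configures homing movement, and hits call ExplodeNetworked.
; An authority-gated explosion chain with impulse, particles and sound is left unconnected.
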(event EventOnObstacleHit
  (params (ImpactPoint :type Vector :default "0, 0, 0") (ImpactNormal :type Vector :default "0, 0, 0"))
  (CallFunction|ExplodeNetworked ImpactPoint))

(event EventBeginPlay
  (bind _asmy_character (Utilities|Casting|CastToMyCharacter (Game|GetPlayerCharacter 0)))
  (bind (_outactors _returnvalue) (Class|KismetSystemLibrary|SphereOverlapActorsNEW (Transformation|GetActorLocation) 1e+04 (Utilities|Array|MakeArray "ObjectTypeQuery3") "/Script/BattleChairs.BattleChairsCharacter" (Utilities|Array|MakeArray _asmy_character)))
  (if _returnvalue
    (for _array_element _outactors
      (bind _asmy_character_2 (Utilities|Casting|CastToMyCharacter _array_element))
      (if (> (Math|Vector|DotProduct (Math|Vector|Normalize (Math|Vector|RotateVector (Math|Vector|MakeVector 1.0 0.0 0.0) (Transformation|GetActorRotation _asmy_character))) (Math|Vector|Normalize (- (Transformation|GetSocketLocation _asmy_character_2 "None") (Transformation|GetActorLocation _asmy_character)))) (Math|Trig|Cos(Degrees) 25.0))
        (Variables|/Script/Engine.ProjectileMovementComponent|SetHomingTargetComponent (Variables|Default|GetProjectileMovement) (Variables|/Script/Engine.Character|GetMesh _asmy_character_2))))))

(fn ConstructionScript
  (bind _projectilemovement (Variables|Default|GetProjectileMovement))
  (Variables|/Script/Engine.ProjectileMovementComponent|SetbIsHomingProjectile _projectilemovement true)
  (Variables|/Script/Engine.ProjectileMovementComponent|SetHomingAccelerationMagnitude _projectilemovement 2e+03)
  (Variables|/Script/Engine.ProjectileMovementComponent|SetInitialSpeed _projectilemovement 1.5e+03))