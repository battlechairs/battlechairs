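; MURICA is an invincibility power-up that temporarily zeroes incoming damage, doubles damage dealt and changes fire rate, plus restores health.
; Any actor overlap spawns smoke and drops the pickup below the level, then buffs player 0 through MyCharacter and BattleChairsCharacter casts.
; Chained delays revert the timed stats after 15 seconds and return the pickup to its BeginPlay transform 45 seconds later, instead of destroying it.
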(event EventActorBeginOverlap
  (params (OtherActor :type Actor%20Object%20Reference))
  (bind _returnvalue (Game|GetPlayerCharacter 0))
  ;[1 1 1] Invincibility Power-Up
  (Effects|SpawnEmitteratLocation "/Game/StarterContent/Particles/P_Smoke.P_Smoke" (Transformation|GetActorLocation))
  (Transformation|AddActorLocalOffset "0,0.000000,-1500.000000" false)
  (bind _asmy_character (Utilities|Casting|CastToMyCharacter _returnvalue))
  (bind _asbattle_chairs_character (Utilities|Casting|CastToBattleChairsCharacter _returnvalue))
  (Variables|/Script/BattleChairs.BattleChairsCharacter|Setfirerate _asbattle_chairs_character 1.0)
  (Variables|/Game/Blueprints/MyCharacter.MyCharacter_C|SetonDamageMult _asmy_character 0.0)
  (Variables|/Game/Blueprints/MyCharacter.MyCharacter_C|SetdamageMult _asmy_character 2.0)
  (Variables|/Game/Blueprints/MyCharacter.MyCharacter_C|SetHealth _asmy_character (+ (Variables|/Game/Blueprints/MyCharacter.MyCharacter_C|GetHealth _asmy_character) (Variables|Default|GethpReturn)))
  (Utilities|FlowControl|Delay 15.0)
  (Variables|/Script/BattleChairs.BattleChairsCharacter|Setfirerate _asbattle_chairs_character 5.0)
  (Variables|/Game/Blueprints/MyCharacter.MyCharacter_C|SetdamageMult _asmy_character 1.0)
  (Variables|/Game/Blueprints/MyCharacter.MyCharacter_C|SetonDamageMult _asmy_character 1.0)
  (Utilities|FlowControl|Delay 45.0)
  (Transformation|SetActorTransform (Variables|Default|GetinitialIPos)))

(event EventBeginPlay
  ;[1 1 1] Invincibility Power-Up
  (Variables|Default|SetinitialIPos (Transformation|GetWorldTransform)))

(fn ConstructionScript)