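; TutorialLookAt is a tutorial Blueprint that sets prompt text from the player's look progress, apparently meant to end in a countdown.
; Each Tick it casts the player character to MyCharacter and compares its Counter to fixed values, showing "Tutorial" at zero, then "Keep Looking!!".
; The countdown checks are nested inside the "Keep Looking!!" equality branch, so the digits are unreachable and a debug "Hello" prints there instead.
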(event EventBeginPlay)

(event EventActorBeginOverlap
  (params (OtherActor :type Actor%20Object%20Reference)))

(event EventTick
  (params (DeltaSeconds :type Float%20%28single-precision%29))
  (bind _asmy_character (Utilities|Casting|CastToMyCharacter (Game|GetPlayerCharacter 0)))
  (if (== 0 (Variables|/Game/Blueprints/MyCharacter.MyCharacter_C|GetCounter _asmy_character))
    (Rendering|Components|TextRender|SetText "Tutorial")
    (elif (== 20 (Variables|/Game/Blueprints/MyCharacter.MyCharacter_C|GetCounter _asmy_character))
      (Rendering|Components|TextRender|SetText "Keep Looking!!")
      (if (== 60 (Variables|/Game/Blueprints/MyCharacter.MyCharacter_C|GetCounter _asmy_character))
        (Rendering|Components|TextRender|SetText (Utilities|String|ToString(Integer) 3))
        (if (== 120 (Variables|/Game/Blueprints/MyCharacter.MyCharacter_C|GetCounter _asmy_character))
          (Rendering|Components|TextRender|SetText (Utilities|String|ToString(Integer) 2))
          (if (== 180 (Variables|/Game/Blueprints/MyCharacter.MyCharacter_C|GetCounter _asmy_character))
            (Rendering|Components|TextRender|SetText (Utilities|String|ToString(Integer) 1))))
        (else
          (Development|PrintString "Hello"))))))

(fn ConstructionScript)