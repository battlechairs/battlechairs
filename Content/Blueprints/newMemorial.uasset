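; Memorial sign actor that changes its displayed text according to the player character's CounterMem value.
; Tick uses OptVar as a frame counter to throttle the check to every 30th tick, then casts player 0 to MyCharacter and reads CounterMem.
; A value of 0 shows "Lincoln Memorial" and 2 shows "Keep Looking!!", while any other value leaves the text unchanged.
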(event EventBeginPlay)

(event EventActorBeginOverlap
  (params (OtherActor :type Actor%20Object%20Reference)))

(event EventTick
  (params (DeltaSeconds :type Float%20%28single-precision%29))
  (Variables|Default|SetoptVar (+ 1 (Variables|Default|GetoptVar)))
  (if (>= (Variables|Default|GetoptVar) 30)
    (Variables|Default|SetoptVar 0)
    (bind _asmy_character (Utilities|Casting|CastToMyCharacter (Game|GetPlayerCharacter 0)))
    (if (== 0 (Variables|/Game/Blueprints/MyCharacter.MyCharacter_C|GetcounterMem _asmy_character))
      (Rendering|Components|TextRender|SetText "Lincoln Memorial")
      (elif (== 2 (Variables|/Game/Blueprints/MyCharacter.MyCharacter_C|GetcounterMem _asmy_character))
        (Rendering|Components|TextRender|SetText "Keep Looking!!")))))

(fn ConstructionScript)