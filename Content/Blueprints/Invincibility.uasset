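; Invincibility power-up pickup that makes the player's MyCharacter temporarily invincible, then respawns.
; Any actor overlap spawns smoke, drops the pickup far below its spot and sets the Invincible flag on player 0's character, without checking who overlapped.
; Chained delays clear the flag, then later restore the transform saved at BeginPlay, hiding the pickup by relocation instead of destroying it.
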(event EventActorBeginOverlap
  (params (OtherActor :type Actor%20Object%20Reference))
  ;[1 1 1] Invincibility Power-Up
  (Effects|SpawnEmitteratLocation "/Game/StarterContent/Particles/P_Smoke.P_Smoke" (Transformation|GetActorLocation))
  (Transformation|AddActorLocalOffset "0,0.000000,-1500.000000" false)
  (bind _asmy_character (Utilities|Casting|CastToMyCharacter (Game|GetPlayerCharacter 0)))
  (Variables|/Game/Blueprints/MyCharacter.MyCharacter_C|SetInvincible _asmy_character (Variables|Default|GetTrue))
  (Utilities|FlowControl|Delay 15.0)
  (Variables|/Game/Blueprints/MyCharacter.MyCharacter_C|SetInvincible _asmy_character (Variables|Default|GetFalse))
  (Utilities|FlowControl|Delay 2e+01)
  (Transformation|SetActorTransform (Variables|Default|GetinitialIPos)))

(event EventBeginPlay
  ;[1 1 1] Invincibility Power-Up
  (Variables|Default|SetinitialIPos (Transformation|GetWorldTransform)))

(fn ConstructionScript)