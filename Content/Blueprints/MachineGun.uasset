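; MachineGun is a replicated-play projectile Blueprint that explodes on its first bounce and deals radial bullet damage.
; On the server, the bounce destroys components, fires a RadialForce impulse and calls ApplyBulletDamage, which damages pawns found by a sphere overlap.
; It then passes itself to player 0's MyCharacter through DestroyActorGlobal for removal.
; The construction script creates a dynamic material instance and calls Play.
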(event OnProjectileBounce(ProjectileMovement)
  (params (ImpactResult :type Hit%20Result%20Structure%20%28by%20ref%29) (ImpactVelocity :type Vector%20%28by%20ref%29 :default "0, 0, 0"))
  (Networking|SwitchHasAuthority
    (:Authority
      ;[1 1 1] Makes the projectile explode and emit an explosion/sound and then damage
      (Components|DestroyComponent)
      (Components|DestroyComponent)
      (Utilities|FlowControl|DoOnce false
        (:Completed
          (Class|RadialForceComponent|FireImpulse (Variables|Default|GetRadialForce))
          (CallFunction|ApplyBulletDamage)
          (bind _asmy_character (Utilities|Casting|CastToMyCharacter (Game|GetPlayerCharacter 0)))
          (Default|DestroyActorGlobal _asmy_character self))))))

(fn ConstructionScript
  (Rendering|Material|CreateDynamicMaterialInstance 0 0 :!class /Script/Engine.PrimitiveComponent)
  (Audio|Components|Audio|Play 0.0))

(fn ApplyBulletDamage
  (bind _outactors (Class|KismetSystemLibrary|SphereOverlapActorsNEW 0 (Transformation|GetActorLocation) (Variables|Default|Getbullet%20radius) (Utilities|Array|MakeArray "ObjectTypeQuery3")))
  (for _array_element _outactors
    (Game|Damage|ApplyDamage _array_element (Variables|Default|GetBulletDamage) (Game|GetInstigatorController) self)
    (Components|DestroyComponent)
    (Utilities|FlowControl|DoOnce false
      (:Completed
        (Class|RadialForceComponent|FireImpulse (Variables|Default|GetRadialForce))))))