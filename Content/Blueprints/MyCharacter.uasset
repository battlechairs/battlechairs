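; Player character that flies on three thrusters, with toggleable lasers, laser vision and server-authoritative health.
; Tick forces flying movement and fluid friction, feeds thruster values into particle parameters and HUD variables, and crossfades low and high looping audio by peak thrust.
; When enabled, laser vision line-traces from camera rotation every tick to damage pawns.
; Damage reduces health on the server, destroying the actor at zero, while OnRep updates the HP text.
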(event OnAudioFinished(ThrusterHigh)
  ;[1 1 1] Thruster Volume
  (Audio|Components|Audio|Play 0.0))

(event OnAudioFinished(ThrusterLow)
  ;[1 1 1] Thruster Volume
  (Audio|Components|Audio|Play 0.0))

(event EventAnyDamage
  (params (Damage :type Float%20%28single-precision%29) (DamageType :type Damage%20Type%20Object%20Reference) (InstigatedBy :type Controller%20Object%20Reference) (DamageCauser :type Actor%20Object%20Reference))
  ;[1 1 1] handle the damages - cant have delay in functions so this stays for now
  (if (Variables|Default|GetInvincible)
    (Utilities|FlowControl|Delay 0 5.0))
  (CallFunction|OnTakeDamage (Variables|Default|GetDamage)))

(event EventBeginPlay
  ;[1 1 1] Init char attributes on server
  (Networking|SwitchHasAuthority
    (:Authority
      (CallFunction|InitAttributes)
      (bind _asprojectile (Utilities|Casting|CastToProjectile (Variables|Default|GetWeapon))
        (:then
          (Variables|Default|SetWeapon _asprojectile))
        (:CastFailed
          _))
      (Components|Activation|Deactivate))))

(event EventTick
  (params (DeltaSeconds :type Float%20%28single-precision%29))
  (bind _returnvalue (Transformation|GetActorRotation))
  (bind _returnvalue_2 (Transformation|GetWorldRotation))
  (bind _one (Variables|Default|Getone))
  (bind _returnvalue_3 (Math|Rotator|Delta(Rotator) _returnvalue_2 _returnvalue))
  (bind _returnvalue_4 (Math|Rotator|GetRotationXVector _returnvalue_3))
  ;[1 1 1] Thrusters
  (if (> (Variables|Default|GetthrusterF) _one)
    (Components|Activation|Activate false)
    (else
      (Components|Activation|Deactivate)))
  (if (> (Variables|Default|GetthrusterL) _one)
    (Components|Activation|Activate false)
    (else
      (Components|Activation|Deactivate)))
  (if (> (Variables|Default|GetthrusterR) _one)
    (Components|Activation|Activate false)
    (else
      (Components|Activation|Deactivate)))
  (Effects|Components|ParticleSystem|SetFloatParameter "ThrusterRate" (* (Variables|Default|GetthrusterF) 2.0))
  (Effects|Components|ParticleSystem|SetVectorParameter "ThrusterVel" (Variables|Default|GetthrusterFV))
  (Effects|Components|ParticleSystem|SetFloatParameter "ThrusterRate" (* (Variables|Default|GetthrusterL) 2.0))
  (Effects|Components|ParticleSystem|SetVectorParameter "ThrusterVel" (Variables|Default|GetthrusterLV))
  (Effects|Components|ParticleSystem|SetFloatParameter "ThrusterRate" (* (Variables|Default|GetthrusterR) 2.0))
  (Effects|Components|ParticleSystem|SetVectorParameter "ThrusterVel" (Variables|Default|GetthrusterRV))
  ;[1 1 1] Enable Z Axis Movement
  (Pawn|Components|CharacterMovement|SetMovementMode "MOVE_Flying" 0)
  ;[1 1 1] disable the "ice skating" effect
  (Variables|/Script/Engine.PhysicsVolume|SetFluidFriction (Class|MovementComponent|GetPhysicsVolume (Pawn|GetMovementComponent)) 1.5)
  ;[1 1 1] Set HUD values
  (Variables|Default|SetthrusterFVal (Variables|Default|GetthrusterF))
  (Variables|Default|SetthrusterLVal (Variables|Default|GetthrusterL))
  (Variables|Default|SetthrusterRVal (Variables|Default|GetthrusterR))
  ;[1 1 1] Thruster Volume
  (CallFunction|SetThrusterVolume)
  ;[1 1 1] Organizing
  (if (Variables|Default|GetlaserVision)
    (Effects|Components|ParticleSystem|SetVectorParameter "CameraView" _returnvalue_4)
    (bind (_outhit _returnvalue_5) (Collision|LineTraceForObjects 0 (Transformation|GetActorLocation) (* _returnvalue_4 5e+03) (Utilities|Array|MakeArray "ObjectTypeQuery3" "ObjectTypeQuery3") false 0 "None"))
    (if _returnvalue_5
      (Game|Damage|ApplyDamage (.HitActor (Collision|BreakHitResult _outhit)) 0.05 (Game|GetInstigatorController) self))))

(event Input|ActionEvents|InputActionToggleLasers
  (:Pressed
    (if (Variables|Default|GetLasersOn)
      (Variables|Default|SetLasersOn false)
      (Components|Activation|Deactivate)
      (Components|Activation|Deactivate)
      (else
        (Variables|Default|SetLasersOn true)
        (Components|Activation|Activate false)
        (Components|Activation|Activate false)))))

(event Input|MouseEvents|LeftMouseButton
  (:Pressed
    (Components|Activation|Activate false))
  (:Released
    (Components|Activation|Deactivate)))

(event Input|MouseEvents|RightMouseButton
  (:Pressed
    (Components|Activation|Activate false))
  (:Released
    (Components|Activation|Deactivate)))

(fn ConstructionScript)

(fn InitAttributes
  (Networking|SwitchHasAuthority
    (:Authority
      (CallFunction|InitHealth))))

(fn InitHealth
  (Variables|Default|SetHealth (Variables|Default|GetMaxHealth)))

(fn UpdateCharDisplayText
  (bind _health (Variables|Default|GetHealth))
  (Rendering|Components|TextRender|SetText (Variables|Default|GetCharText) (Utilities|String|BuildString(Float) "" "HP" _health))
  (Variables|Default|SetPlayerHealth _health))

(fn OnTakeDamage
  (params (Damage :type Float%20%28single-precision%29))
  (Networking|SwitchHasAuthority
    (:Authority
      (Variables|Default|SetHealth (- (Variables|Default|GetHealth) Damage))
      (if (<= (Variables|Default|GetHealth) 0.0)
        (Actor|DestroyActor)))))

(fn OnRepHealth
  (CallFunction|UpdateCharDisplayText))

(fn SetThrusterVolume
  (bind _thrusterf (Variables|Default|GetthrusterF))
  (bind _thrusterl (Variables|Default|GetthrusterL))
  (bind _thrusterr (Variables|Default|GetthrusterR))
  (bind _returnvalue (Math|Float|Max(Float) _thrusterf _thrusterl _thrusterr))
  (bind _returnvalue_2 (/ _returnvalue 1.5))
  (if (> _returnvalue_2 1.0)
    (Audio|Components|Audio|SetVolumeMultiplier (- _returnvalue_2 1.0) :!class /Script/Engine.AudioComponent)
    (Audio|Components|Audio|SetVolumeMultiplier (- 2.0 _returnvalue_2) :!class /Script/Engine.AudioComponent)
    (else
      (Audio|Components|Audio|SetVolumeMultiplier (* _returnvalue_2 0.0) :!class /Script/Engine.AudioComponent)
      (Audio|Components|Audio|SetVolumeMultiplier (* _returnvalue_2 1.0) :!class /Script/Engine.AudioComponent))))