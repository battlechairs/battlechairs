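; Mushroom pickup actor that temporarily grows the player character when overlapped, then respawns.
; On overlap it spawns a fire particle effect, drops itself far below its spot to hide, and scales MyCharacter up fivefold.
; After timed delays it restores the character's scale, then returns the mushroom to the transform saved at BeginPlay.
; The overlapping actor is not checked; the effect always targets player 0.
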(event EventBeginPlay
  (Variables|Default|SetinitialMPos (Transformation|GetWorldTransform)))

(event EventActorBeginOverlap
  (params (OtherActor :type Actor%20Object%20Reference))
  (Effects|SpawnEmitteratLocation "/Game/StarterContent/Particles/P_Fire.P_Fire" (Transformation|GetActorLocation))
  (Transformation|AddActorLocalOffset "0, 0,-1500.000000" false)
  (bind _asmy_character (Utilities|Casting|CastToMyCharacter (Game|GetPlayerCharacter 0)))
  (Transformation|SetActorRelativeScale3D _asmy_character "5.000000,5.000000,5.000000")
  (Utilities|FlowControl|Delay 15.0)
  (Transformation|SetActorRelativeScale3D _asmy_character "1.000000,1.000000,1.000000")
  (Utilities|FlowControl|Delay 3e+01)
  (Transformation|SetActorTransform (Variables|Default|GetinitialMPos)))

(fn ConstructionScript)